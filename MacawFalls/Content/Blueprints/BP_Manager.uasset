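; BP_Manager is a manager Blueprint that looks up the start transform for a numbered player.
; SpawnPlayers loops over the Players array and compares each PlayerStartTag with a name built from "Player" and PlayerInt.
; It stores the transform of a matching actor in PlayerTransform, but despite its name it does not spawn anything.
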(fn `SpawnPlayers`
  (for _array_element (`self.Players`)
    (bind _output (`|ConvertAsset` _array_element))
    (if (== (`PlayerStart.PlayerStartTag` _output) (`KismetStringLibrary.Conv_StringToName` (`KismetStringLibrary.Concat_StrStr` "Player" (`KismetStringLibrary.Conv_IntToString` (`self.PlayerInt`)))))
      (set `self.PlayerTransform` (`self.GetTransform` _output)))))

(fn `UserConstructionScript`)