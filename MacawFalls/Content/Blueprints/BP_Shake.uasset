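; Trigger volume that plays a cave-collapse effect while a BP_Character is inside it.
; On BeginPlay it spawns a falling-rock emitter at the Manager's RockStartLocation and keeps it deactivated.
; Overlap begin shakes the Manager's camera, activates the rocks and starts a 2D collapse sound; overlap end stops all three.
; An Active flag prevents repeated triggering, and the rock emitter is reused rather than respawned.
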(event `self.ReceiveBeginPlay`
  (`self.SpawnRocks`)
  (`ActorComponent.Deactivate` (`self.RockEmitter`)))

(event `SpawnRocks`
  (bind _output (`|ConvertAsset` (`/Game/Blueprints/BP_Manager.RockStartLocation` (`|ConvertAsset` (`self.Manager`)))))
  (bind _returnvalue (`GameplayStatics.SpawnEmitterAtLocation` "/Game/VFX/FallingRocks/P_FallingRock.P_FallingRock" (`self.K2_GetActorLocation` _output) (`self.K2_GetActorRotation` _output) (1.0 1.0 1.0) false))
  (set `self.RockEmitter` _returnvalue))

(event `self.Collision.OnComponentBeginOverlap`
  (params (OverlappedComponent :type "PrimitiveComponent Object Reference") (OtherActor :type "Actor Object Reference") (OtherComp :type "PrimitiveComponent Object Reference") (OtherBodyIndex :type Integer) (bFromSweep :type Boolean) (SweepResult :type "HitResult Structure (by ref)"))
  (cast `/Game/Character/BP_Character` OtherActor)
  (if (not (`self.Active`))
    (set `self.Active` true)
    (`/Game/Blueprints/BP_Camera.Shake` (`|ConvertAsset` (`/Game/Blueprints/BP_Manager.Camera` (`|ConvertAsset` (`self.Manager`)))))
    (`ActorComponent.Activate` (`self.RockEmitter`) false)
    (bind _returnvalue (`GameplayStatics.SpawnSound2D` "/Game/Sounds/Cave_Collapse_-_Sound_Effect__320_kbps_.Cave_Collapse_-_Sound_Effect__320_kbps_" 1.0 1.0 0.0 null))
    (set `self.CollapseSound` _returnvalue)))

(event `self.Collision.OnComponentEndOverlap`
  (params (OverlappedComponent :type "PrimitiveComponent Object Reference") (OtherActor :type "Actor Object Reference") (OtherComp :type "PrimitiveComponent Object Reference") (OtherBodyIndex :type Integer))
  (cast `/Game/Character/BP_Character` OtherActor)
  (if (`self.Active`)
    (set `self.Active` false)
    (`/Game/Blueprints/BP_Camera.StopShake` (`|ConvertAsset` (`/Game/Blueprints/BP_Manager.Camera` (`|ConvertAsset` (`self.Manager`)))))
    (`ActorComponent.Deactivate` (`self.RockEmitter`))
    (bind _collapsesound (`self.CollapseSound`)
      (:`then`
        (`ActorComponent.K2_DestroyComponent` _collapsesound))
      (:`else`))))

(fn `UserConstructionScript`)