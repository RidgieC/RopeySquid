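; BP_GameMode is a game mode that sets up two local players and their characters when play begins.
; Spawner first creates both players, then for each index sets PlayerInt on a Manager object and calls its SpawnPlayers.
; It spawns a BP_Character at the Manager's PlayerTransform, has the matching player controller possess it, copies the index onto it and adds it to the Manager's PlayerCharacters.
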(event `self.ReceiveBeginPlay`
  (`self.Spawner`))

(fn `Spawner`
  (bind _output (`|ConvertAsset` (`self.Manager`)))
  (for _index (range 2)
    (`GameplayStatics.CreatePlayer` _index))
  (for _index_2 (range 2)
    (bind _output_get (set `/Game/Blueprints/BP_Manager.PlayerInt` _index_2 _output))
    (`/Game/Blueprints/BP_Manager.SpawnPlayers` _output)
    (bind _returnvalue (`|SpawnActorFromClass` "/Game/Character/BP_Character.BP_Character_C" (`/Game/Blueprints/BP_Manager.PlayerTransform` _output) "Undefined" "OverrideRootScale" null null))
    (`Controller.Possess` (`GameplayStatics.GetPlayerController` _output_get) _returnvalue)
    (set `/Game/Character/BP_Character.PlayerInt` _output_get _returnvalue)
    (`KismetArrayLibrary.Array_Add` (`/Game/Blueprints/BP_Manager.PlayerCharacters` (`|ConvertAsset` (`self.Manager`))) (`|ConvertAsset` _returnvalue))))

(fn `UserConstructionScript`)