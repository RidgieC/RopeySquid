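; BP_Camera is a two-player shared camera that zooms with the distance between the players.
; Shortly after BeginPlay it takes the first two player characters from a Manager and caches start positions.
; Each tick it moves a Box to the players' midpoint and interpolates spring arm length toward their distance, capped at 800.
; SetCameraPosition is an empty stub, and the cached positions are never used in live logic.
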(event `self.ReceiveBeginPlay`
  (bind _playercharacters (`/Game/Blueprints/BP_Manager.PlayerCharacters` (`|ConvertAsset` (`self.Manager`))))
  (`KismetSystemLibrary.Delay` 0.2)
  (`|ExecutionSequence`
    (:`then_0`
      (set `self.Player1` (`|ConvertAsset` (`|GetArrayItem` _playercharacters)))
      (set `self.Player2` (`|ConvertAsset` (`|GetArrayItem` _playercharacters 1)))
      (set `self.CameraStartPosition` (`self.K2_GetActorLocation`))
      (set `self.Setup` true))
    (:`then_1`
      (set `self.CameraXPosition` (.x (`SceneComponent.K2_GetComponentLocation` (`self.SpringArm`)))))
    (:`then_2`
      (set `self.CameraYPosition` (.y (`SceneComponent.K2_GetComponentLocation` (`self.SpringArm`)))))
    (:`then_3`
      (set `self.CameraZPosition` (.z (`SceneComponent.K2_GetComponentLocation` (`self.SpringArm`)))))))

(event `self.ReceiveTick`
  (params (DeltaSeconds :type "Float (single-precision)"))
  (set `self.Delta Seconds` DeltaSeconds)
  (`|ExecutionSequence`
    (:`then_0`
      (if (`self.Setup`)
        (`self.DistanceBetweenPlayers`)
        (`self.CenterCamera`)
        (`self.CameraZoom`)
        (`self.SetBoxPosition`)))))

(event `DistanceBetweenPlayers`
  (set `self.PlayerDistance` (`self.GetDistanceTo` (`self.Player1`) (`self.Player2`))))

(event `CenterCamera`
  (set `self.CenterPosition` (/ (+ (`self.K2_GetActorLocation` (`self.Player1`)) (`self.K2_GetActorLocation` (`self.Player2`))) 2.0)))

(event `CameraZoom`
  (bind _springarm (`self.SpringArm`))
  (set `SpringArmComponent.TargetArmLength` (`KismetMathLibrary.FInterpTo` (`SpringArmComponent.TargetArmLength` _springarm) (`KismetMathLibrary.FMax` (`KismetMathLibrary.FMin` (`self.PlayerDistance`) 800.0) -500.0) (`self.Delta Seconds`) 1.0) _springarm))

(event `SetBoxPosition`
  (`SceneComponent.K2_SetWorldLocation` (`self.Box`) (`self.CenterPosition`) false false))

(event `SetCameraPosition`)

(fn `UserConstructionScript`)